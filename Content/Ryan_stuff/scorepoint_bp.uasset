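; Score point Blueprint where the player drops off carried artifacts to earn points.
; Four artifact meshes start hidden on BeginPlay, each paired with its own collision component.
; When a Ryan_chracter_edit holding an artifact overlaps one, its Score increments, its held artifact is cleared and hidden, and that slot's artifact becomes visible.
; The four handlers are duplicated logic, and none checks whether its slot is already filled.
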(event OnComponentBeginOverlap(collision1)
  (params (OverlappedComponent :type Primitive%20Component%20Object%20Reference) (OtherActor :type Actor%20Object%20Reference) (OtherComp :type Primitive%20Component%20Object%20Reference) (OtherBodyIndex :type Integer) (bFromSweep :type Boolean) (SweepResult :type Hit%20Result%20Structure%20%28by%20ref%29))
  ;[1 1 1] messy collisoion code
  (bind _asryan_chracter_edit (Utilities|Casting|CastToRyan_chracter_edit OtherActor))
  (if (Variables|/Game/Ryan_stuff/Ryan_chracter_edit.Ryan_chracter_edit_C|Getartifact%20hold _asryan_chracter_edit)
    (Math|Integer|IncrementInt (Variables|/Game/Ryan_stuff/Ryan_chracter_edit.Ryan_chracter_edit_C|Getscore _asryan_chracter_edit)
      (:%20%20
        (Variables|/Game/Ryan_stuff/Ryan_chracter_edit.Ryan_chracter_edit_C|Setartifact%20hold _asryan_chracter_edit false)
        (Rendering|SetVisibility (Variables|/Game/Ryan_stuff/Ryan_chracter_edit.Ryan_chracter_edit_C|Getartifact _asryan_chracter_edit) false false)
        (Rendering|SetVisibility (Variables|Default|Getartifact1) true false)))))

(event OnComponentBeginOverlap(collision2)
  (params (OverlappedComponent :type Primitive%20Component%20Object%20Reference) (OtherActor :type Actor%20Object%20Reference) (OtherComp :type Primitive%20Component%20Object%20Reference) (OtherBodyIndex :type Integer) (bFromSweep :type Boolean) (SweepResult :type Hit%20Result%20Structure%20%28by%20ref%29))
  ;[1 1 1] messy collisoion code
  (bind _asryan_chracter_edit (Utilities|Casting|CastToRyan_chracter_edit OtherActor))
  (if (Variables|/Game/Ryan_stuff/Ryan_chracter_edit.Ryan_chracter_edit_C|Getartifact%20hold _asryan_chracter_edit)
    (Math|Integer|IncrementInt (Variables|/Game/Ryan_stuff/Ryan_chracter_edit.Ryan_chracter_edit_C|Getscore _asryan_chracter_edit)
      (:%20%20
        (Variables|/Game/Ryan_stuff/Ryan_chracter_edit.Ryan_chracter_edit_C|Setartifact%20hold _asryan_chracter_edit false)
        (Rendering|SetVisibility (Variables|/Game/Ryan_stuff/Ryan_chracter_edit.Ryan_chracter_edit_C|Getartifact _asryan_chracter_edit) false false)
        (Rendering|SetVisibility (Variables|Default|Getartifact2) true false)))))

(event OnComponentBeginOverlap(collision4)
  (params (OverlappedComponent :type Primitive%20Component%20Object%20Reference) (OtherActor :type Actor%20Object%20Reference) (OtherComp :type Primitive%20Component%20Object%20Reference) (OtherBodyIndex :type Integer) (bFromSweep :type Boolean) (SweepResult :type Hit%20Result%20Structure%20%28by%20ref%29))
  ;[1 1 1] messy collisoion code
  (bind _asryan_chracter_edit (Utilities|Casting|CastToRyan_chracter_edit OtherActor))
  (if (Variables|/Game/Ryan_stuff/Ryan_chracter_edit.Ryan_chracter_edit_C|Getartifact%20hold _asryan_chracter_edit)
    (Math|Integer|IncrementInt (Variables|/Game/Ryan_stuff/Ryan_chracter_edit.Ryan_chracter_edit_C|Getscore _asryan_chracter_edit)
      (:%20%20
        (Variables|/Game/Ryan_stuff/Ryan_chracter_edit.Ryan_chracter_edit_C|Setartifact%20hold _asryan_chracter_edit false)
        (Rendering|SetVisibility (Variables|/Game/Ryan_stuff/Ryan_chracter_edit.Ryan_chracter_edit_C|Getartifact _asryan_chracter_edit) false false)
        (Rendering|SetVisibility (Variables|Default|Getartifact4) true false)))))

(event OnComponentBeginOverlap(collision3)
  (params (OverlappedComponent :type Primitive%20Component%20Object%20Reference) (OtherActor :type Actor%20Object%20Reference) (OtherComp :type Primitive%20Component%20Object%20Reference) (OtherBodyIndex :type Integer) (bFromSweep :type Boolean) (SweepResult :type Hit%20Result%20Structure%20%28by%20ref%29))
  ;[1 1 1] messy collisoion code
  (bind _asryan_chracter_edit (Utilities|Casting|CastToRyan_chracter_edit OtherActor))
  (if (Variables|/Game/Ryan_stuff/Ryan_chracter_edit.Ryan_chracter_edit_C|Getartifact%20hold _asryan_chracter_edit)
    (Math|Integer|IncrementInt (Variables|/Game/Ryan_stuff/Ryan_chracter_edit.Ryan_chracter_edit_C|Getscore _asryan_chracter_edit)
      (:%20%20
        (Variables|/Game/Ryan_stuff/Ryan_chracter_edit.Ryan_chracter_edit_C|Setartifact%20hold _asryan_chracter_edit false)
        (Rendering|SetVisibility (Variables|/Game/Ryan_stuff/Ryan_chracter_edit.Ryan_chracter_edit_C|Getartifact _asryan_chracter_edit) false false)
        (Rendering|SetVisibility (Variables|Default|Getartifact3) true false)))))

(event EventBeginPlay
  ;[1 1 1] visibility disable
  (Utilities|FlowControl|Sequence
    (:then_0
      (Rendering|SetVisibility (Variables|Default|Getartifact1) false false))
    (:then_1
      (Rendering|SetVisibility (Variables|Default|Getartifact2) false false))
    (:then_2
      (Rendering|SetVisibility (Variables|Default|Getartifact3) false false))
    (:then_3
      (Rendering|SetVisibility (Variables|Default|Getartifact4) false false))))

(fn ConstructionScript)
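; Firepit prop for the Low Poly Viking World set, combining a static mesh, a point light and a fire particle effect.
; The construction script applies exposed variables to the light's intensity, units, color, radius, shadows and visibility.
; It also sets the mesh material and toggles the particle fire.
; The event graph holds no active logic, so there is no runtime behavior.
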(event EventBeginPlay)

(event Collision|EventActorBeginOverlap
  (params (OtherActor :type Actor%20Object%20Reference)))

(event EventTick
  (params (DeltaSeconds :type Float%20%28single-precision%29)))

(fn ConstructionScript
  (Rendering|Components|Light|SetIntensity (Variables|Default|GetPointLight) (Variables|Default|GetLight_Intensity))
  (Rendering|Components|Light|SetLightColor (Variables|Default|GetPointLight) (Variables|Default|GetLight_Color) true)
  (Rendering|Lighting|SetAttenuationRadius (Variables|Default|GetPointLight) (Variables|Default|GetAttenuation%20Radius))
  (Rendering|SetVisibility (Variables|Default|GetPointLight) (Variables|Default|GetAffects_World) true)
  (Class|LocalLightComponent|SetIntensityUnits (Variables|Default|GetPointLight) (Variables|Default|GetLight_Intensity_Units))
  (Rendering|Components|Light|SetCastShadows (Variables|Default|GetPointLight) (Variables|Default|GetCast_Shadows))
  (Rendering|Material|SetMaterial (Variables|Default|GetSM_Firepit_02) 0 (Variables|Default|GetMaterial))
  (Rendering|SetVisibility (Variables|Default|GetParticles) (Variables|Default|GetParticle_Fire) true))
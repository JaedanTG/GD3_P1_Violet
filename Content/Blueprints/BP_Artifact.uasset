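; BP_Artifact is a collectible artifact that a BP_Player picks up by overlapping its Box.
; The overlap runs only on authority while uncollected and, as written, requires both the player's IsMonster and ArtifactHeld flags to be true.
; Pickup marks it collected, sets ArtifactHeld, shows the player's held artifact and hides the Cube through a custom visibility event.
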(event OnComponentBeginOverlap(Box)
  (params (OverlappedComponent :type Primitive%20Component%20Object%20Reference) (OtherActor :type Actor%20Object%20Reference) (OtherComp :type Primitive%20Component%20Object%20Reference) (OtherBodyIndex :type Integer) (bFromSweep :type Boolean) (SweepResult :type Hit%20Result%20Structure%20%28by%20ref%29))
  (Networking|SwitchHasAuthority
    (:Authority
      (if (not (Variables|Default|GetCollected))
        (bind _asbp_player (Utilities|Casting|CastToBP_Player OtherActor))
        (if (and (!= (Variables|/Game/Blueprints/BP_Player.BP_Player_C|GetIsMonster _asbp_player) false) (!= (Variables|/Game/Blueprints/BP_Player.BP_Player_C|GetArtifactHeld _asbp_player) false))
          (Variables|Default|SetCollected true)
          (Variables|/Game/Blueprints/BP_Player.BP_Player_C|SetArtifactHeld _asbp_player true)
          (Default|SetHeldArtifactVisibility _asbp_player true)
          (CallFunction|ShowHideCollectibleArtifact false))))))

(event Custom|ShowHideCollectibleArtifact
  (params (Visibility :type Boolean))
  (Rendering|SetVisibility (Variables|Default|GetCube) Visibility false))

(fn ConstructionScript)
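; BP_Key is a pickup key that a non-monster player collects by overlapping its box.
; On the authority, the overlap marks the key collected and stores it as the player's held key, provided the player holds none.
; It then hides the cube mesh through SetKeyVisibility and plays a pickup sound on the player.
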(event OnComponentBeginOverlap(Box)
  (params (OverlappedComponent :type Primitive%20Component%20Object%20Reference) (OtherActor :type Actor%20Object%20Reference) (OtherComp :type Primitive%20Component%20Object%20Reference) (OtherBodyIndex :type Integer) (bFromSweep :type Boolean) (SweepResult :type Hit%20Result%20Structure%20%28by%20ref%29))
  (Networking|SwitchHasAuthority
    (:Authority
      (if (not (Variables|Default|GetCollected))
        (bind _asbp_player (Utilities|Casting|CastToBP_Player OtherActor))
        (if (and (== (Variables|/Game/Blueprints/BP_Player.BP_Player_C|GetIsMonster _asbp_player) false) (== (Variables|/Game/Blueprints/BP_Player.BP_Player_C|GetIsKeyHeld _asbp_player) false))
          (Variables|Default|SetCollected true)
          (Variables|/Game/Blueprints/BP_Player.BP_Player_C|SetIsKeyHeld _asbp_player true)
          (Variables|/Game/Blueprints/BP_Player.BP_Player_C|SetHeldKey _asbp_player self)
          (CallFunction|SetKeyVisibility false)
          (Default|PlaySound _asbp_player "/Game/Audio/sell_buy_item.sell_buy_item" 0.5))))))

(event Custom|SetKeyVisibility
  (params (Visibility :type Boolean))
  (Rendering|SetVisibility (Variables|Default|GetCube) Visibility false))

(event EventBeginPlay)

(fn ConstructionScript)
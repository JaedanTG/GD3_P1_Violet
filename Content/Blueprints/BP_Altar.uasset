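; BP_Altar is the altar where players return carried artifacts to one of four slots.
; Each slot's collision overlap runs ReturnArtifact on the server only, for a BP_Player holding an artifact.
; That function clears the player's held artifact, shows the slot's artifact through SetArtifactSlotVisibility, and increments the returned-artifact count in GI_Main2.
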(event OnComponentBeginOverlap(collision1)
  (params (OverlappedComponent :type Primitive%20Component%20Object%20Reference) (OtherActor :type Actor%20Object%20Reference) (OtherComp :type Primitive%20Component%20Object%20Reference) (OtherBodyIndex :type Integer) (bFromSweep :type Boolean) (SweepResult :type Hit%20Result%20Structure%20%28by%20ref%29))
  ;[1 1 1] messy collisoion code
  (Networking|SwitchHasAuthority
    (:Authority
      (CallFunction|ReturnArtifact OtherActor (Variables|Default|Getartifact1)))))

(event OnComponentBeginOverlap(collision2)
  (params (OverlappedComponent :type Primitive%20Component%20Object%20Reference) (OtherActor :type Actor%20Object%20Reference) (OtherComp :type Primitive%20Component%20Object%20Reference) (OtherBodyIndex :type Integer) (bFromSweep :type Boolean) (SweepResult :type Hit%20Result%20Structure%20%28by%20ref%29))
  ;[1 1 1] messy collisoion code
  (Networking|SwitchHasAuthority
    (:Authority
      (CallFunction|ReturnArtifact OtherActor (Variables|Default|Getartifact2)))))

(event OnComponentBeginOverlap(collision4)
  (params (OverlappedComponent :type Primitive%20Component%20Object%20Reference) (OtherActor :type Actor%20Object%20Reference) (OtherComp :type Primitive%20Component%20Object%20Reference) (OtherBodyIndex :type Integer) (bFromSweep :type Boolean) (SweepResult :type Hit%20Result%20Structure%20%28by%20ref%29))
  ;[1 1 1] messy collisoion code
  (Networking|SwitchHasAuthority
    (:Authority
      (CallFunction|ReturnArtifact OtherActor (Variables|Default|Getartifact4)))))

(event OnComponentBeginOverlap(collision3)
  (params (OverlappedComponent :type Primitive%20Component%20Object%20Reference) (OtherActor :type Actor%20Object%20Reference) (OtherComp :type Primitive%20Component%20Object%20Reference) (OtherBodyIndex :type Integer) (bFromSweep :type Boolean) (SweepResult :type Hit%20Result%20Structure%20%28by%20ref%29))
  ;[1 1 1] messy collisoion code
  (Networking|SwitchHasAuthority
    (:Authority
      (CallFunction|ReturnArtifact OtherActor (Variables|Default|Getartifact3)))))

(event Custom|SetArtifactSlotVisibility
  (params (ArtifactSlot :type Scene%20Component%20Object%20Reference) (Visibility :type Boolean))
  (Rendering|SetVisibility ArtifactSlot Visibility false))

(event EventBeginPlay)

(fn ConstructionScript)

(fn ReturnArtifact
  (params (OverlappedActor :type Object%20Object%20Reference) (ArtifactSlot :type Scene%20Component%20Object%20Reference))
  (bind _asbp_player (Utilities|Casting|CastToBP_Player OverlappedActor))
  (if (Variables|/Game/Blueprints/BP_Player.BP_Player_C|GetArtifactHeld _asbp_player)
    (Variables|/Game/Blueprints/BP_Player.BP_Player_C|SetArtifactHeld _asbp_player false)
    (Default|SetHeldArtifactVisibility _asbp_player false)
    (CallFunction|SetArtifactSlotVisibility ArtifactSlot true)
    (bind _asgi_main_2 (Utilities|Casting|CastToGI_Main2 (Game|GetGameInstance)))
    (Default|IncrementReturnedArtifacts _asgi_main_2)))
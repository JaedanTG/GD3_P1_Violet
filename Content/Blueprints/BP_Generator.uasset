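; BP_Generator is a world actor that non-monster players disable by touching it once its linked Lockbox is unlocked, removing a linked Barrier.
; The server checks the Box overlap, flags the generator as Destroyed, hides its Cube through the SetGeneratorVisibility event and destroys the Barrier.
; Tick stops the generator audio every frame while Destroyed or DisableSound is set.
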(event OnComponentBeginOverlap(Box)
  (params (OverlappedComponent :type Primitive%20Component%20Object%20Reference) (OtherActor :type Actor%20Object%20Reference) (OtherComp :type Primitive%20Component%20Object%20Reference) (OtherBodyIndex :type Integer) (bFromSweep :type Boolean) (SweepResult :type Hit%20Result%20Structure%20%28by%20ref%29))
  (Networking|SwitchHasAuthority
    (:Authority
      (Utilities|IsValid (Variables|Default|GetLockbox)
        (:Is%20Valid
          (if (and (== (Variables|Default|GetDestroyed) false) (Variables|/Game/Blueprints/BP_Box.BP_Box_C|GetUnlocked (Variables|Default|GetLockbox)))
            (bind _asbp_player (Utilities|Casting|CastToBP_Player OtherActor))
            (if (== (Variables|/Game/Blueprints/BP_Player.BP_Player_C|GetIsMonster _asbp_player) false)
              (Variables|Default|SetDestroyed true)
              (CallFunction|SetGeneratorVisibility false)
              (Actor|DestroyActor (Variables|Default|GetBarrier)))))))))

(event Custom|SetGeneratorVisibility
  (params (Visibility :type Boolean))
  (Rendering|SetVisibility (Variables|Default|GetCube) Visibility false))

(event EventTick
  (params (DeltaSeconds :type Float%20%28single-precision%29))
  (if (or (Variables|Default|GetDestroyed) (Variables|Default|GetDisableSound))
    (Audio|Components|Audio|Stop (Variables|Default|GetAudio))))

(fn ConstructionScript)